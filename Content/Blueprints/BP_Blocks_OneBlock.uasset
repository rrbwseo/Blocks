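; A single colored block actor that reports hand overlaps to its BlockMapManager.
; Init stores the manager and color, and applies the color through a dynamic M_Color material instance on BlockMesh.
; BoxCollision overlap events compare OverlappedComponent with the pawn's left and right hand meshes to set that hand's overlapped block on the manager.
; End overlap resets it to EmptyOneBlock only if it still references this block.
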(event `self.BoxCollision.OnComponentBeginOverlap`
  (params (OverlappedComponent :type "PrimitiveComponent Object Reference") (OtherActor :type "Actor Object Reference") (OtherComp :type "PrimitiveComponent Object Reference") (OtherBodyIndex :type Integer) (bFromSweep :type Boolean) (SweepResult :type "HitResult Structure (by ref)"))
  (bind _blockmapmanager (`self.BlockMapManager`))
  (bind _pawn (`/Game/Blueprints/BP_BlockMapManager.Pawn` (`self.BlockMapManager`)))
  (if (== OverlappedComponent (`/Game/Blueprints/VR_Pawn.LeftHandStaticMesh` _pawn))
    (set `/Game/Blueprints/BP_BlockMapManager.LeftHandOverlapedOneBlock` self _blockmapmanager)
    (elif (== OverlappedComponent (`/Game/Blueprints/VR_Pawn.RightHandStaticMesh` _pawn))
      (set `/Game/Blueprints/BP_BlockMapManager.RightHandOverlapedOneBlock` self _blockmapmanager))))

(event `self.BoxCollision.OnComponentEndOverlap`
  (params (OverlappedComponent :type "PrimitiveComponent Object Reference") (OtherActor :type "Actor Object Reference") (OtherComp :type "PrimitiveComponent Object Reference") (OtherBodyIndex :type Integer))
  (bind _blockmapmanager (`self.BlockMapManager`))
  (bind _blockmapmanager_2 (`self.BlockMapManager`))
  (bind _pawn (`/Game/Blueprints/BP_BlockMapManager.Pawn` (`self.BlockMapManager`)))
  (if (== OverlappedComponent (`/Game/Blueprints/VR_Pawn.LeftHandStaticMesh` _pawn))
    (if (== (`/Game/Blueprints/BP_BlockMapManager.LeftHandOverlapedOneBlock` (`self.BlockMapManager`)) self)
      (set `/Game/Blueprints/BP_BlockMapManager.LeftHandOverlapedOneBlock` (`/Game/Blueprints/BP_BlockMapManager.EmptyOneBlock` _blockmapmanager_2) _blockmapmanager_2))
    (elif (== OverlappedComponent (`/Game/Blueprints/VR_Pawn.RightHandStaticMesh` _pawn))
      (if (== (`/Game/Blueprints/BP_BlockMapManager.RightHandOverlapedOneBlock` (`self.BlockMapManager`)) self)
        (set `/Game/Blueprints/BP_BlockMapManager.RightHandOverlapedOneBlock` (`/Game/Blueprints/BP_BlockMapManager.EmptyOneBlock` _blockmapmanager) _blockmapmanager)))))

(fn `Init`
  (params (Color :type "LinearColor Structure") (BlockMapManager :type "/Game/Blueprints/BP_BlockMapManager Object Reference"))
  (bind _output_get (set `self.Color` Color))
  (bind _returnvalue (`PrimitiveComponent.CreateDynamicMaterialInstance` (`self.BlockMesh`) 0 "/Game/Materials/M_Color.M_Color"))
  (`MaterialInstanceDynamic.SetVectorParameterValue` _returnvalue "Color" _output_get)
  (set `self.Material` _returnvalue)
  (set `self.BlockMapManager` BlockMapManager))

(fn `UserConstructionScript`
  (`parent.UserConstructionScript`))