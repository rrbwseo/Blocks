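; Manager actor for a VR block scene that spawns a row of six colored BP_Blocks_OneBlock pieces at fixed world positions on BeginPlay.
; SpawnLostBlock switches on a type index to spawn one color, initializes it with a reference to this manager, and stores it in a per-color variable and the OneBlocks array.
; BeginPlay also caches the VR_Pawn and resets both hand-attached block references to EmptyOneBlock.
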(event `self.ReceiveBeginPlay`
  (`|ExecutionSequence`
    (:`then_0`
      (bind _asvr_pawn (cast `/Game/Blueprints/VR_Pawn` (`GameplayStatics.GetPlayerPawn` 0)))
      (set `self.Pawn` _asvr_pawn))
    (:`then_1`
      (`self.SpawnLostBlock` 0)
      (`self.SpawnLostBlock` 1)
      (`self.SpawnLostBlock` 2)
      (`self.SpawnLostBlock` 3)
      (`self.SpawnLostBlock` 4)
      (`self.SpawnLostBlock` 5)
      (set `self.LeftHandAttachedOneBlock` (`self.EmptyOneBlock`))
      (set `self.RightHandAttachedOneBlock` (`self.EmptyOneBlock`)))))

(fn `SpawnLostBlock`
  (params (BlockType :type Integer))
  (switch `int` BlockType
    (:`0`
      (bind _returnvalue (`|SpawnActorFromClass` "/Game/Blueprints/BP_Blocks_OneBlock.BP_Blocks_OneBlock_C" (`KismetMathLibrary.MakeTransform` (150.0 100.0 130.0)) "Undefined" "OverrideRootScale"))
      (`/Game/Blueprints/BP_Blocks_OneBlock.Init` _returnvalue (struct :`R` 1.0 :`A` 1.0) self)
      (bind _output_get (set `self.OneBlockRed` _returnvalue))
      (`KismetArrayLibrary.Array_Add` (`self.OneBlocks`) _output_get))
    (:`1`
      (bind _returnvalue_2 (`|SpawnActorFromClass` "/Game/Blueprints/BP_Blocks_OneBlock.BP_Blocks_OneBlock_C" (`KismetMathLibrary.MakeTransform` (150.0 60.0 130.0)) "Undefined" "OverrideRootScale"))
      (`/Game/Blueprints/BP_Blocks_OneBlock.Init` _returnvalue_2 (struct :`R` 1.0 :`G` 1.0 :`A` 1.0) self)
      (bind _output_get_2 (set `self.OneBlockYellow` _returnvalue_2))
      (`KismetArrayLibrary.Array_Add` (`self.OneBlocks`) _output_get_2))
    (:`2`
      (bind _returnvalue_3 (`|SpawnActorFromClass` "/Game/Blueprints/BP_Blocks_OneBlock.BP_Blocks_OneBlock_C" (`KismetMathLibrary.MakeTransform` (150.0 20.0 130.0)) "Undefined" "OverrideRootScale"))
      (`/Game/Blueprints/BP_Blocks_OneBlock.Init` _returnvalue_3 (struct :`B` 1.0 :`A` 1.0) self)
      (bind _output_get_3 (set `self.OneBlockBlue` _returnvalue_3))
      (`KismetArrayLibrary.Array_Add` (`self.OneBlocks`) _output_get_3))
    (:`3`
      (bind _returnvalue_4 (`|SpawnActorFromClass` "/Game/Blueprints/BP_Blocks_OneBlock.BP_Blocks_OneBlock_C" (`KismetMathLibrary.MakeTransform` (150.0 -20.0 130.0)) "Undefined" "OverrideRootScale"))
      (`/Game/Blueprints/BP_Blocks_OneBlock.Init` _returnvalue_4 (struct :`G` 1.0 :`A` 1.0) self)
      (bind _output_get_4 (set `self.OneBlockGreen` _returnvalue_4))
      (`KismetArrayLibrary.Array_Add` (`self.OneBlocks`) _output_get_4))
    (:`4`
      (bind _returnvalue_5 (`|SpawnActorFromClass` "/Game/Blueprints/BP_Blocks_OneBlock.BP_Blocks_OneBlock_C" (`KismetMathLibrary.MakeTransform` (150.0 -60.0 130.0)) "Undefined" "OverrideRootScale"))
      (`/Game/Blueprints/BP_Blocks_OneBlock.Init` _returnvalue_5 (struct :`R` 1.0 :`G` 1.0 :`B` 1.0 :`A` 1.0) self)
      (bind _output_get_5 (set `self.OneBlockWhite` _returnvalue_5))
      (`KismetArrayLibrary.Array_Add` (`self.OneBlocks`) _output_get_5))
    (:`5`
      (bind _returnvalue_6 (`|SpawnActorFromClass` "/Game/Blueprints/BP_Blocks_OneBlock.BP_Blocks_OneBlock_C" (`KismetMathLibrary.MakeTransform` (150.0 -100.0 130.0)) "Undefined" "OverrideRootScale"))
      (`/Game/Blueprints/BP_Blocks_OneBlock.Init` _returnvalue_6 (struct :`A` 1.0) self)
      (bind _output_get_6 (set `self.OneBlockBlack` _returnvalue_6))
      (`KismetArrayLibrary.Array_Add` (`self.OneBlocks`) _output_get_6))))

(fn `UserConstructionScript`)